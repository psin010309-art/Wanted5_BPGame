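; BP_CharacterStat is a character stat component that tracks current HP and signals when it runs out.
; On BeginPlay it sets CurrentHp to MaxHp from its Data asset, if that asset is valid.
; ReceiveDamage subtracts damage clamped at zero and broadcasts the OnHpZero dispatcher whenever the result is zero, including on repeated hits at zero.
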(event `self.ReceiveBeginPlay`
  ;[0.674 1 0.7353 0.5] 시작하면 데이터에 설정된 HP로 세팅
  (bind _data (`self.Data`) ; 데이터 에셋이 설정될 때 읽을 수 있게
    (:`then`
      (set `self.CurrentHp` (`/Game/Blueprints/Game/Data/BP_CharacterData.MaxHp` _data)))
    (:`else`)))

(event `ReceiveDamage`
  (params (Damage :type "Float (double-precision)"))
  ;[1 0.4859 0.9086 0.5] 데미지 처리 및 이벤트 발행
  (bind _output_get (set `self.CurrentHp` (`KismetMathLibrary.FMax` (- (`self.CurrentHp`) Damage))))
  (if (== _output_get 0.0)
    (`self.OnHpZero`) ; hp가 0 됐다고 방송해줌
  ))