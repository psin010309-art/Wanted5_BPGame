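; BP_Cow is a toy cow gimmick that launches a player character upward on contact and explodes when damaged.
; A dynamic material instance switches the body color while any actor overlaps the Box, then restores it on exit.
; Player-tagged Characters entering the Box receive a vertical velocity-change impulse scaled by PushPower.
; Any damage disables the Box collision, destroys the actor and spawns a scaled-up explosion emitter.
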(event `self.ReceiveBeginPlay`
  (bind _returnvalue (`PrimitiveComponent.CreateDynamicMaterialInstance` (`self.StaticMesh`) 0 "/Game/Toycow/M_ToyCow.M_ToyCow" "None"))
  (bind _output_get (set `self.MaterialInstance` _returnvalue))
  (`MaterialInstanceDynamic.SetVectorParameterValue` _output_get "BodyColor" (`self.OriginColor`)))

(event `self.Box.OnComponentBeginOverlap`
  (params (OverlappedComponent :type "PrimitiveComponent Object Reference") (OtherActor :type "Actor Object Reference") (OtherComp :type "PrimitiveComponent Object Reference") (OtherBodyIndex :type Integer) (bFromSweep :type Boolean) (SweepResult :type "HitResult Structure (by ref)"))
  (`MaterialInstanceDynamic.SetVectorParameterValue` (`self.MaterialInstance`) "BodyColor" (`self.CollideColor`))
  (if (`self.ActorHasTag` OtherActor "Player")
    (bind _ascharacter (cast `Character` OtherActor)) ; 캐릭터 타입으로 형변환 노드
    (`CharacterMovementComponent.AddImpulse` (`Character.CharacterMovement` _ascharacter) (* (`KismetMathLibrary.MakeVector` 0.0 0.0 1.0) (`self.PushPower`)) true)))

(event `self.Box.OnComponentEndOverlap`
  (params (OverlappedComponent :type "PrimitiveComponent Object Reference") (OtherActor :type "Actor Object Reference") (OtherComp :type "PrimitiveComponent Object Reference") (OtherBodyIndex :type Integer))
  (`MaterialInstanceDynamic.SetVectorParameterValue` (`self.MaterialInstance`) "BodyColor" (`self.OriginColor`)))

(event `self.ReceiveAnyDamage`
  (params (Damage :type "Float (single-precision)") (DamageType :type "DamageType Object Reference") (InstigatedBy :type "Controller Object Reference") (DamageCauser :type "Actor Object Reference"))
  ;[0.15 0.1143 0.01528 0.5] 대미지 처리
  (`PrimitiveComponent.SetCollisionEnabled` (`self.Box`) "NoCollision")
  (`self.K2_DestroyActor`)
  (`GameplayStatics.SpawnEmitterAtLocation` "/Game/Particles/P_Explosion.P_Explosion" (`self.K2_GetActorLocation`) (struct) (10.0 10.0 10.0)))

(fn `UserConstructionScript`)