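; Level streaming trigger actor that loads its TargetLevel sublevel when an actor tagged Player overlaps it.
; The load blocks and starts hidden, then the streaming level is looked up by the soft reference's object name and set visible.
; On EndPlay it unloads that level with blocking, but only if the trigger itself carries the Player tag, as no other actor is checked there.
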(event `self.ReceiveActorBeginOverlap`
  (params (OtherActor :type "Actor Object Reference"))
  (if (`self.ActorHasTag` OtherActor "Player")
    (`GameplayStatics.LoadStreamLevelBySoftObjectPtr` (`self.TargetLevel`) false true)
    (set `LevelStreaming.bShouldBeVisible` true (`GameplayStatics.GetStreamingLevel` (`KismetStringLibrary.Conv_StringToName` (`KismetSystemLibrary.GetObjectName` (`|ConvertAsset` (`self.TargetLevel`))))))))

(event `self.ReceiveEndPlay`
  (params (EndPlayReason :type "EEndPlayReason Enum" :default "Destroyed"))
  (if (`self.ActorHasTag` "Player")
    (`GameplayStatics.UnloadStreamLevelBySoftObjectPtr` (`self.TargetLevel`) true)))

(fn `UserConstructionScript`)